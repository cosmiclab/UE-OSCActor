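; An actor whose visibility is controlled remotely over OSC.
; On BeginPlay it binds an address built from its OSCActorComponent's object name through BP_OscManagerActor, with a handler that reads a bool.
; SetVisibility applies that state to the actor, its static mesh components and a "Hidden" tag.
; Tick also reapplies changes to the Visible variable and, optionally, copies the hidden state to all attached actors recursively.
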(event EventBeginPlay
  (bind _returnvalue (Actor|GetActorOfClass "/Game/CosmicLab/Zepp/Blueprints/OSC/BP_OscManagerActor.BP_OscManagerActor_C"))
  (Class|OscManagerActor|BindEventtoAllServers _returnvalue (Utilities|String|Append "/Operation/OscActor/Visible/" (Variables|/Script/OSCActor.OSCActorComponent|GetObjectName (Variables|Default|GetOSCActorComponent))) (EventDispatchers|CreateEvent :!event OnSetVisibility))
  (CallFunction|SetVisibility (Variables|OSCActor|GetbVisible)))

(event EventUpdatefromOSC)

(event EventTick
  (params (DeltaSeconds :type Float%20%28single-precision%29))
  (if (Variables|Default|GetbControlChildVisibility)
    (for _array_element (Actor|GetAttachedActors true true)
      (Rendering|SetActorHiddenInGame _array_element (Variables|Default|GetbHidden))))
  (if (!= (Variables|OSCActor|GetbVisible) (Variables|OSCActor|GetbOldVisible))
    (CallFunction|SetVisibility (Variables|OSCActor|GetbVisible))))

(fn ConstructionScript)

(fn SetVisibility
  (params (bNewVisiblity :type Boolean))
  (bind _output_get (Variables|OSCActor|SetbVisible bNewVisiblity))
  (bind _output_get_2 (Variables|OSCActor|SetbOldVisible _output_get))
  (if _output_get_2
    (Utilities|Array|RemoveItem (Variables|Default|GetTags) "Hidden")
    (else
      (Utilities|Array|Add (Variables|Default|GetTags) "Hidden")))
  (Variables|Default|SetTags (Variables|Default|GetTags))
  (Utilities|FlowControl|Sequence
    (:then_0
      (Rendering|SetActorHiddenInGame (not (Variables|OSCActor|GetbVisible))))
    (:then_1
      (for _array_element (Actor|GetComponentsByClass "/Script/Engine.StaticMeshComponent")
        (Development|SetHiddeninGame _array_element (not (Variables|OSCActor|GetbVisible)) false)))))

(fn OnSetVisibility
  (params (AddressPattern :type OSC%20Address%20Structure%20%28by%20ref%29) (Message :type OSC%20Message%20Structure%20%28by%20ref%29) (IPAddress :type String) (Port :type Integer))
  (bind _value (Class|OSCManager|GetBool Message))
  (CallFunction|SetVisibility _value)
  (return))