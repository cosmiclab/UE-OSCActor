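; Base OSC actor Blueprint that adds fade-in and fade-out to actor show/hide.
; HideActor calls SetVisibility, which either snaps the fade value and hidden state or sets a target through StartFade.
; Tick moves the value linearly over FadeTime, calling the empty UpdateFade hook for child classes to apply it.
; A timed fade reaching zero sets hidden to false, leaving the actor unhidden, unlike the zero-time path.
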(event EventTick
  (params (DeltaSeconds :type Float%20%28single-precision%29))
  (|CallParentFunction DeltaSeconds)
  (if (!= (Variables|Default|GetFadeCurrent) (Variables|Default|GetFadeTarget))
    (if (== (Variables|Default|GetFadeTime) 0.0)
      (bind _output_get (Variables|Default|SetFadeCurrent (Variables|Default|GetFadeTarget)))
      (Rendering|SetActorHiddenInGame (Math|Float|NearlyEqual(Float) _output_get 0.0 1e-06))
      (else
        (bind _fadecurrent (CallFunction|UpdateFadeValue DeltaSeconds))
        (CallFunction|UpdateFade)
        (if (Math|Float|NearlyEqual(Float) _fadecurrent 0.0 1e-06)
          (Rendering|SetActorHiddenInGame false))))))

(event EventHideActor
  (params (bNewHidden :type Boolean) (bFade :type Boolean))
  (CallFunction|SetVisibility (not bNewHidden) bFade))

(fn ConstructionScript
  (|CallParentFunction))

(fn InitializeFade
  (bind _output_get (Variables|Default|SetFadeCurrent (Math|Float|SelectFloat 1.0 0.0 (Variables|Default|GetbHidden))))
  (Variables|Default|SetFadeTarget _output_get))

(fn StartFade
  (params (bVisible :type Boolean))
  (if bVisible
    (Variables|Default|SetFadeTarget 1.0)
    (Rendering|SetActorHiddenInGame false)
    (else
      (Variables|Default|SetFadeTarget 0.0))))

(fn UpdateFade)

(fn SetVisibility
  (params (bVisible :type Boolean) (bFade :type Boolean))
  (bind _returnvalue (not bVisible))
  (if bFade
    (CallFunction|StartFade bVisible)
    (else
      (bind _output_get (Variables|Default|SetFadeCurrent (Math|Float|SelectFloat 0.0 1.0 _returnvalue)))
      (Variables|Default|SetFadeTarget _output_get)
      (CallFunction|UpdateFade)
      (Rendering|SetActorHiddenInGame _returnvalue))))

(fn UpdateFadeValue
  (params (DeltaSeconds :type Float%20%28double-precision%29))
  (bind _value (CallFunction|MoveTowards (Variables|Default|GetFadeCurrent) (Variables|Default|GetFadeTarget) (/ DeltaSeconds (Variables|Default|GetFadeTime))))
  (bind _output_get (Variables|Default|SetFadeCurrent _value))
  (return _output_get))